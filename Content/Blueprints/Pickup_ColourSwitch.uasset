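; Colour-switch pickup that changes the slime player's colour to match its own.
; On overlap with a Slime_Player of a different colour, it calls the slime's UpdateColour, then hides its sphere for two seconds without disabling collision.
; A slime already of the same colour triggers nothing.
; The construction script applies the material for the selected colour, so edits preview live in the editor.
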(event `self.ReceiveActorBeginOverlap`
  (params (OtherActor :type "Actor Object Reference"))
  ;[1 1 1] Changes colour of the slime to the same colour as the pickup and dissapears for 2 seconds. If the colour is the same, does nothing.
  (bind _asslime_player (cast `/Game/Player/Slime_Player` OtherActor))
  (if (not (`|EnumEquality` (`self.Switcher_CurrentColour`) (`/Game/Player/Slime_Player.Slime_CurrentColour` _asslime_player)))
    (`/Game/Player/Slime_Player.Update Colour` _asslime_player (`self.Switcher_CurrentColour`))
    (`SceneComponent.SetVisibility` (`self.Sphere`) false false)
    (`KismetSystemLibrary.Delay` 2.0)
    (`SceneComponent.SetVisibility` (`self.Sphere`) true false)))

(fn `UpdateColour`
  (params (`New Colour` :type "/Game/Enumurators/Colour_List Enum" :default "NewEnumerator3"))
  ;[1 1 1] Changes Colour of Pickup
  (bind _output_get (set `self.Switcher_CurrentColour` `New Colour`))
  (switch `/Game/Enumurators/Colour_List` _output_get
    (:`NewEnumerator3`
      (`PrimitiveComponent.SetMaterial` (`self.Sphere`) 0 "/Game/Textures/Materials/Green1.Green1"))
    (:`NewEnumerator0`
      (`PrimitiveComponent.SetMaterial` (`self.Sphere`) 0 "/Game/Textures/Materials/Red.Red"))
    (:`NewEnumerator1`
      (`PrimitiveComponent.SetMaterial` (`self.Sphere`) 0 "/Game/Textures/Materials/Blue.Blue"))
    (:`NewEnumerator2`
      (`PrimitiveComponent.SetMaterial` (`self.Sphere`) 0 "/Game/Textures/Materials/Yellow.Yellow"))
    (:`NewEnumerator4`
      (`PrimitiveComponent.SetMaterial` (`self.Sphere`) 0 "/Game/Textures/Materials/Pink.Pink"))
    (:`NewEnumerator5`
      (`PrimitiveComponent.SetMaterial` (`self.Sphere`) 0 "/Game/Textures/Materials/Purple.Purple"))
    (:`NewEnumerator6`
      (`PrimitiveComponent.SetMaterial` (`self.Sphere`) 0 "/Game/Textures/Materials/Orange.Orange"))))

(fn `UserConstructionScript`
  ;[1 1 1] Updates Colour Live
  (`self.UpdateColour` (`self.Switcher_CurrentColour`)))