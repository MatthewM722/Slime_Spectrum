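; GooGate is a coloured gate that lets a Slime_Player through only when the slime's colour matches its own.
; The construction script calls UpdateColour, which sets the gate's material from GateCurrentColour.
; On overlap it compares that colour to the player's SlimeCurrentColour, disabling Gate collision on a match and restoring it otherwise.
; An older per-colour boolean check is left unconnected, and its SetMaterialGooGate helper is never called here.
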(event `self.ReceiveActorBeginOverlap`
  (params (OtherActor :type "Actor Object Reference"))
  ;[1 1 1] Matthews Colour Gate
  (bind _asslime_player (cast `/Game/Player/Slime_Player` OtherActor))
  (if (`|EnumEquality` (`self.Gate_CurrentColour`) (`/Game/Player/Slime_Player.Slime_CurrentColour` _asslime_player))
    (`PrimitiveComponent.SetCollisionEnabled` (`self.Gate`) "NoCollision")
    (else
      (`PrimitiveComponent.SetCollisionEnabled` (`self.Gate`) "QueryAndPhysics"))))

(fn `SetMaterial(GooGate)`
  (if (== (`PrimitiveComponent.GetMaterial` (`self.Gate`) 0) "/Game/Textures/Materials/Red.Red")
    (set `self.redGate` true)
    (elif (== (`PrimitiveComponent.GetMaterial` (`self.Gate`) 0) "/Game/Textures/Materials/Blue.Blue")
      (set `self.blueGate` true)
      (elif (== (`PrimitiveComponent.GetMaterial` (`self.Gate`) 0) "/Game/Textures/Materials/Yellow.Yellow")
        (set `self.yellowGate` true)
        (elif (== (`PrimitiveComponent.GetMaterial` (`self.Gate`) 0) "/Game/Textures/Materials/Green.Green")
          (set `self.greenGate` true)
          (elif (== (`PrimitiveComponent.GetMaterial` (`self.Gate`) 0) "/Game/Textures/Materials/Pink.Pink")
            (set `self.pinkGate` true)
            (elif (== (`PrimitiveComponent.GetMaterial` (`self.Gate`) 0) "/Game/Textures/Materials/Purple.Purple")
              (set `self.purpleGate` true)
              (elif (== (`PrimitiveComponent.GetMaterial` (`self.Gate`) 0) "/Game/Textures/Materials/Orange.Orange")
                (set `self.orangeGate` true)))))))))

(fn `Update Colour`
  (params (`New Colour` :type "/Game/Enumurators/Colour_List Enum" :default "NewEnumerator3"))
  ;[1 1 1] Changes Colour of Gate
  (bind _output_get (set `self.Gate_CurrentColour` `New Colour`))
  (switch `/Game/Enumurators/Colour_List` _output_get
    (:`NewEnumerator3`
      (`PrimitiveComponent.SetMaterial` (`self.Gate`) 0 "/Game/Textures/Materials/Green1.Green1"))
    (:`NewEnumerator0`
      (`PrimitiveComponent.SetMaterial` (`self.Gate`) 0 "/Game/Textures/Materials/Red.Red"))
    (:`NewEnumerator1`
      (`PrimitiveComponent.SetMaterial` (`self.Gate`) 0 "/Game/Textures/Materials/Blue.Blue"))
    (:`NewEnumerator2`
      (`PrimitiveComponent.SetMaterial` (`self.Gate`) 0 "/Game/Textures/Materials/Yellow.Yellow"))
    (:`NewEnumerator4`
      (`PrimitiveComponent.SetMaterial` (`self.Gate`) 0 "/Game/Textures/Materials/Pink.Pink"))
    (:`NewEnumerator5`
      (`PrimitiveComponent.SetMaterial` (`self.Gate`) 0 "/Game/Textures/Materials/Purple.Purple"))
    (:`NewEnumerator6`
      (`PrimitiveComponent.SetMaterial` (`self.Gate`) 0 "/Game/Textures/Materials/Orange.Orange"))))

(fn `UserConstructionScript`
  (`self.Update Colour` (`self.Gate_CurrentColour`)))